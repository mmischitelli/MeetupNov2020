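; BP_MN2GameMode is a game mode that tracks score, top score, enemy count and kills.
; On BeginPlay it sets game-only input, shows the HUD widget and plays the soundtrack.
; Update functions adjust the counters, and GameOver shows its widget with the cursor and UI-only input.
; LoadScore and SaveScore are called at begin and end of play but are empty, so nothing persists.
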(event `self.ReceiveBeginPlay`
  (`WidgetBlueprintLibrary.SetInputMode_GameOnly` (`GameplayStatics.GetPlayerController` 0))
  (`self.LoadScore`)
  (`self.UpdateScore` 0)
  (bind _returnvalue (`|CreateWidget` "/Game/Blueprints/UI/BPW_HUD.BPW_HUD_C"))
  (bind _output_get (set `self.BPW_Score` _returnvalue))
  (`UserWidget.AddToViewport` _output_get 0)
  (`GameplayStatics.PlaySound2D` "/Game/Assets/SoundFX/soundtrack.soundtrack" 1.0 1.0 0.0 null null))

(event `self.ReceiveEndPlay`
  (params (EndPlayReason :type "EEndPlayReason Enum" :default "Destroyed"))
  (`self.SaveScore`))

(fn `GameOver`
  (bind _returnvalue (`GameplayStatics.GetPlayerController` 0))
  (bind _returnvalue_2 (`|CreateWidget` "/Game/Blueprints/UI/BPW_GameOver.BPW_GameOver_C"))
  (`UserWidget.AddToViewport` _returnvalue_2 0)
  (set `PlayerController.bShowMouseCursor` true _returnvalue)
  (`WidgetBlueprintLibrary.SetInputMode_UIOnlyEx` _returnvalue _returnvalue_2))

(fn `Increment Killed Enemies Counter Fn`
  (bind _result (`/Engine/EditorBlueprintResources/StandardMacros.IncrementInt` (`self.KilledEnemies`))
    (:`  `
      (set `self.KilledEnemies` _result)
      (`self.UpdateEnemyCount` -1))))

(fn `LoadScore`)

(fn `SaveScore`)

(fn `UpdateEnemyCount`
  (params (HowManyToAdd :type Integer))
  (set `self.EnemyCount` (+ HowManyToAdd (`self.EnemyCount`))))

(fn `UpdateScore`
  (params (Amount :type Integer))
  (bind _output_get (set `self.Score` (+ Amount (`self.Score`))))
  (if (>= _output_get (`self.TopScore`))
    (set `self.TopScore` (`self.Score`))))

(fn `UserConstructionScript`)