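; Player spaceship for the MN2 game, which rises and spins in on spawn before it can fire.
; Axis input eases vertical and horizontal speeds, applied as swept moves each Tick with yaw following sideways speed; non-projectile hits bounce the ship off.
; Looping timers repeat single primary and paired secondary projectiles while held.
; Damage drains health; at zero the ship explodes, calls GameOver on the game mode and destroys itself.
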(event `self.ReceiveBeginPlay`
  (bind _spawnlocation (`self.SpawnLocation`))
  ;[1 1 1] Spawn animation
  (bind _asbp_mn2game_mode (cast `/Game/Blueprints/BP_MN2GameMode` (`GameplayStatics.GetGameMode`)))
  (set `self.BP_MN2GameMode` _asbp_mn2game_mode)
  (set `self.Yaw` (.yaw (`self.K2_GetActorRotation`)))
  (set `self.SpawnLocation` (`self.K2_GetActorLocation`))
  (bind (_direction _speed) (`Timeline|Spawn Animation`)
    (:`Update`
      (`|ExecutionSequence`
        (:`then_0`
          (`self.K2_SetActorLocation` (`KismetMathLibrary.VLerp` _spawnlocation (+ _spawnlocation (`KismetMathLibrary.MakeVector` 0.0 0.0 (`self.SpawnMovementOffset`))) _speed)))
        (:`then_1`
          (`SceneComponent.K2_SetRelativeRotation` (`self.SpaceshipMesh`) (`KismetMathLibrary.RLerp` (struct) (`KismetMathLibrary.MakeRotator` 0.0 0.0 (+ (`self.Yaw`) (* (`KismetMathLibrary.Conv_IntToDouble` (`self.SpawnSpinCount`)) 360.0))) _speed) false false))))
    (:`Finished`
      (set `self.IsMoveable` true))))

(event `InputAxis|MoveUpDown`
  (params (AxisValue :type "Float (single-precision)"))
  ;[1 1 1] Player input
  (bind _interpolatedspeed (`self.CalcMovementAmount` AxisValue (`self.VerticalSpeed`)))
  (set `self.VerticalSpeed` _interpolatedspeed))

(event `InputAxis|MoveLeftRight`
  (params (AxisValue :type "Float (single-precision)"))
  ;[1 1 1] Player input
  (bind _interpolatedspeed (`self.CalcMovementAmount` AxisValue (`self.HorizontalSpeed`)))
  (set `self.HorizontalSpeed` _interpolatedspeed))

(event `self.ReceiveTick`
  (params (DeltaSeconds :type "Float (single-precision)"))
  ;[1 1 1] Movement
  (set `self.DeltaSecs` DeltaSeconds)
  (`self.K2_SetActorLocation` (+ (`self.K2_GetActorLocation`) (`KismetMathLibrary.MakeVector` 0.0 (`self.HorizontalSpeed`))) true)
  (`self.K2_SetActorLocation` (+ (`self.K2_GetActorLocation`) (`KismetMathLibrary.MakeVector` 0.0 0.0 (`self.VerticalSpeed`))) true)
  (`/Engine/EditorBlueprintResources/StandardMacros.IsValid` self
    (:`Is Valid`
      (`SceneComponent.K2_SetRelativeRotation` (`self.SpaceshipMesh`) (`KismetMathLibrary.RInterpTo_Constant` (`SceneComponent.RelativeRotation` (`self.SpaceshipMesh`)) (`KismetMathLibrary.MakeRotator` 0.0 0.0 (+ (`self.Yaw`) (* (`self.HorizontalSpeed`) -7.0))) (`self.DeltaSecs`) 250.0) false false))))

(event `PrimaryFireFn`
  (bind _returnvalue_location (`KismetMathLibrary.BreakTransform` (`SceneComponent.K2_GetComponentToWorld` (`self.PrimaryFireSpawn`))))
  ;[1 1 1] Primary Fire
  (`self.PrimaryFire` _returnvalue_location :!label _label))

(event `InputAction|Primary`
  (params (Key :type "Key Structure"))
  ;[1 1 1] Primary Fire
  (:`Pressed`
    (if (`self.IsMoveable`)
      (`KismetSystemLibrary.K2_SetTimer` null "PrimaryFireFn" 0.2 true)
      (goto _label)))
  (:`Released`
    (`KismetSystemLibrary.K2_ClearTimer` null "PrimaryFireFn")))

(event `SecondaryFireFn`
  ;[1 1 1] Secondary Fire
  (`self.SecondaryFire` (`|MakeArray` (`SceneComponent.K2_GetComponentToWorld` (`self.SecondaryFireDXSpawn`)) (`SceneComponent.K2_GetComponentToWorld` (`self.SecondaryFireSXSpawn`))) :!label _label_2))

(event `InputAction|Secondary`
  (params (Key :type "Key Structure"))
  ;[1 1 1] Secondary Fire
  (:`Pressed`
    (if (`self.IsMoveable`)
      (`KismetSystemLibrary.K2_SetTimer` null "SecondaryFireFn" 0.3 true)
      (goto _label_2)))
  (:`Released`
    (`KismetSystemLibrary.K2_ClearTimer` null "SecondaryFireFn")))

(event `self.ReceiveAnyDamage`
  (params (Damage :type "Float (single-precision)") (DamageType :type "DamageType Object Reference") (InstigatedBy :type "Controller Object Reference") (DamageCauser :type "Actor Object Reference"))
  (bind _returnvalue (`self.K2_GetActorLocation`))
  ;[1 1 1] Receiving damage & death
  (bind _output_get (set `self.Health` (`KismetMathLibrary.FClamp` (- (`self.Health`) Damage) 0.0 (`self.MaxHealth`))))
  (if (<= _output_get 0.0)
    (`GameplayStatics.SpawnEmitterAtLocation` "/Game/Assets/Particles/P_Pixel_Explosion_Player.P_Pixel_Explosion_Player" _returnvalue)
    (`GameplayStatics.PlaySoundAtLocation` "/Game/Assets/SoundFX/explosion.explosion" _returnvalue (struct) 1.0 1.0 0.0 null null null)
    (`/Game/Blueprints/BP_MN2GameMode.GameOver` (`self.BP_MN2GameMode`))
    (`self.K2_DestroyActor`)))

(event `self.Box.OnComponentHit`
  (params (HitComponent :type "PrimitiveComponent Object Reference") (OtherActor :type "Actor Object Reference") (OtherComp :type "PrimitiveComponent Object Reference") (NormalImpulse :type "Vector Structure") (Hit :type "HitResult Structure (by ref)"))
  ;[1 1 1] Bounce on hit
  (cast `/Game/Blueprints/Projectiles/BP_ProjectileEnemyBase` OtherActor
    (:`CastFailed`
      (set `self.HorizontalSpeed` (* (* (`KismetMathLibrary.Abs` (`self.HorizontalSpeed`)) 3.0) (.y Hit_Normal)))
      (set `self.VerticalSpeed` (* (* (`KismetMathLibrary.Abs` (`self.VerticalSpeed`)) 3.0) (.z Hit_Normal))))))

(fn `CalcMovementAmount`
  (params (Direction :type "Float (double-precision)") (Speed :type "Float (double-precision)"))
  (returns (InterpolatedSpeed :type "Float (double-precision)"))
  (bind _deltasecs (`self.DeltaSecs`))
  (return (`KismetMathLibrary.FInterpTo` Speed (* (* (`self.MovementSpeed`) Direction) _deltasecs) _deltasecs 10.0)))

(fn `PrimaryFire`
  (params (Location :type "Vector Structure"))
  (`|SpawnActorFromClass` "/Game/Blueprints/Projectiles/BP_ProjectilePlayerPrimary.BP_ProjectilePlayerPrimary_C" (`KismetMathLibrary.MakeTransform` Location) "AlwaysSpawn" "OverrideRootScale" null (struct :`G` 0.831373 :`B` 0.94902 :`A` 1.0) self)
  (`GameplayStatics.PlaySoundAtLocation` "/Game/Assets/SoundFX/laser2.laser2" Location (struct) 0.25 1.0 0.0 null null null))

(fn `SecondaryFire`
  (params (Array :type "Array of Transform Structure"))
  (for _array_element Array
    (`|SpawnActorFromClass` "/Game/Blueprints/Projectiles/BP_ProjectilePlayerSecondary.BP_ProjectilePlayerSecondary_C" (`KismetMathLibrary.MakeTransform` (.location _array_element)) "AlwaysSpawn" "OverrideRootScale" null (struct :`R` 0.007499 :`G` 0.89627 :`B` 0.122139 :`A` 1.0) self)
    (`GameplayStatics.PlaySoundAtLocation` "/Game/Assets/SoundFX/laser2.laser2" (.location _array_element) (struct) 0.125 1.0 0.0 null null null)))

(fn `UserConstructionScript`
  (set `self.Health` (`self.MaxHealth`)))