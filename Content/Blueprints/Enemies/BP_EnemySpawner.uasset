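; Enemy spawner actor that, when enabled, feeds standard enemies, bosses and asteroids into the level.
; Two looping one-second timers drive it: one adds randomly delayed enemies under the game mode's cap, plus a boss once per five-kill milestone.
; The other runs a random-count asteroid loop with a Delay inside.
; All spawns use the actor's X and random Y/Z within its collision bounds.
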(event `self.ReceiveBeginPlay`
  ;[1 1 1] Initialization
  (bind _asbp_mn2game_mode (cast `/Game/Blueprints/BP_MN2GameMode` (`GameplayStatics.GetGameMode`)))
  (set `self.BP_GameMode` _asbp_mn2game_mode)
  (if (`self.SpawnerEnabled`)
    (`|ExecutionSequence`
      (:`then_0`
        (`KismetSystemLibrary.K2_SetTimer` null "SpawnEnemyFn" 1.0 true))
      (:`then_1`
        (`KismetSystemLibrary.K2_SetTimer` null "SpawnAsteroidFn" 1.0 true)))))

(event `SpawnEnemyFn`
  (bind _bp_gamemode (`self.BP_GameMode`))
  (bind _returnvalue (`MN2GameMode.GetNumKilledEnemies` _bp_gamemode))
  ;[1 1 1] Spawn Enemies
  (if (< (`MN2GameMode.GetCurrentEnemyCount` _bp_gamemode) (`MN2GameMode.MaxNumOfEnemies` _bp_gamemode))
    (if (and (== (mod _returnvalue 5) 0) (!= _returnvalue (`self.CurrentEnemiesKilled`)))
      (`self.SpawnBossFn`))
    (`KismetSystemLibrary.Delay` (`KismetMathLibrary.RandomFloatInRange` 0.5 2.0))
    (`|SpawnActorFromClass` "/Game/Blueprints/Enemies/BP_EnemyStandard.BP_EnemyStandard_C" (`KismetMathLibrary.MakeTransform` (`self.GetRandomLocation`)) "Undefined" "OverrideRootScale" null null)))

(event `SpawnBossFn`
  ;[1 1 1] Spawn Enemies
  ;;[1 1 1] Spawn Boss
  (set `self.CurrentEnemiesKilled` (`MN2GameMode.GetNumKilledEnemies` (`self.BP_GameMode`)))
  (`|SpawnActorFromClass` "/Game/Blueprints/Enemies/BP_EnemyBoss.BP_EnemyBoss_C" (`KismetMathLibrary.MakeTransform` (`self.GetRandomLocation`)) "Undefined" "OverrideRootScale" null null))

(event `SpawnAsteroidFn`
  ;[1 1 1] Spawn asteroids
  (for _ (range (+ (`KismetMathLibrary.RandomIntegerInRange` 2 5) 1))
    (`KismetSystemLibrary.Delay` (`KismetMathLibrary.RandomFloatInRange` 0.5 2.0))
    (`|SpawnActorFromClass` "/Game/Blueprints/Enemies/BP_EnemyAsteroid.BP_EnemyAsteroid_C" (`KismetMathLibrary.MakeTransform` (`self.GetRandomLocation`)) "Undefined" "OverrideRootScale" null null)))

(fn `GetRandomLocation`
  (returns (Location :type "Vector Structure"))
  (locals (NewLocalVar_0 :type "Vector Structure" :default (0.0 0.0 0.0)))
  (bind _returnvalue_x (`KismetMathLibrary.BreakVector` (`self.K2_GetActorLocation`)))
  (bind (_origin _boxextent) (`KismetSystemLibrary.GetComponentBounds` (`self.CollisionComponent`)))
  (bind (_returnvalue_x_2 _returnvalue_y _returnvalue_z) (`KismetMathLibrary.BreakVector` (`KismetMathLibrary.RandomPointInBoundingBox` _origin _boxextent)))
  (return (`KismetMathLibrary.MakeVector` _returnvalue_x _returnvalue_y _returnvalue_z)))

(fn `UserConstructionScript`)