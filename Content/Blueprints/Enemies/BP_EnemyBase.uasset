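; Base enemy that drops in on spawn via a timeline, then moves sideways along Y at a random speed, reversing on non-projectile hits.
; Tick drives a randomly delayed shot when the player is within Y range, with a signed offset staggering sound and projectile.
; Lethal damage or ramming the player, which deals half its current health, triggers explosion, destruction and GameMode score and kill updates.
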(event `self.ReceiveBeginPlay`
  ;[1 1 1] Initialization
  (bind _asbp_mn2game_mode (cast `/Game/Blueprints/BP_MN2GameMode` (`GameplayStatics.GetGameMode`)))
  (bind _output_get (set `self.BP_GameMode` _asbp_mn2game_mode))
  (`/Game/Blueprints/BP_MN2GameMode.UpdateEnemyCount` _output_get 1)
  (set `self.MoveDirection` (`KismetMathLibrary.RandomBool`))
  (set `self.MoveSpeed` (`KismetMathLibrary.RandomFloatInRange` (`self.MinSpeed`) (`self.MaxSpeed`)))
  (set `self.SpawnLocation` (`self.K2_GetActorLocation`))
  (`self.PlaySpawnAnimationFn`))

(event `PlaySpawnAnimationFn`
  (bind _spawnlocation (`self.SpawnLocation`))
  ;[1 1 1] Spawn Animation
  (bind (_direction _entry_animation) (`Timeline|SpawnAnimation`)
    (:`Update`
      (`self.K2_SetActorLocation` (`KismetMathLibrary.VLerp` _spawnlocation (- _spawnlocation (0.0 0.0 120.0)) _entry_animation)))
    (:`Finished`
      (set `self.MoveEnable` true))))

(event `self.ReceiveTick`
  (params (DeltaSeconds :type "Float (single-precision)"))
  (bind (_returnvalue_x _returnvalue_y) (`KismetMathLibrary.BreakVector` (`self.K2_GetActorLocation`)))
  (bind _returnvalue (`GameplayStatics.GetPlayerPawn` 0))
  (bind _returnvalue_location (`KismetMathLibrary.BreakTransform` (`self.GetTransform`)))
  (bind (_returnvalue_x_2 _returnvalue_y_2) (`KismetMathLibrary.BreakVector` (`self.K2_GetActorLocation` _returnvalue)))
  ;[1 1 1] Movement
  (if (`self.MoveEnable`)
    (`self.K2_SetActorLocation` (+ (`self.K2_GetActorLocation`) (* (`KismetMathLibrary.MakeVector` 0.0 (* (`self.MoveSpeed`) (`KismetMathLibrary.SelectFloat` 1.0 -1.0 (`self.MoveDirection`)))) DeltaSeconds)) true)
    (`/Engine/EditorBlueprintResources/StandardMacros.IsValid` _returnvalue
      (:`Is Valid`
        (`KismetSystemLibrary.Delay` (`KismetMathLibrary.RandomFloatInRange` 0.5 2.0))
        (`/Engine/EditorBlueprintResources/StandardMacros.IsValid` (`GameplayStatics.GetPlayerPawn` 0)
          (:`Is Valid`
            (if (<= (`KismetMathLibrary.Abs` (- _returnvalue_y_2 _returnvalue_y)) (`self.DistanceFromPlayer`))
              (if (>= (`self.ShootSoundOffset`) 0.0)
                (`KismetSystemLibrary.Delay` (`self.ShootSoundOffset`)))
              (`GameplayStatics.PlaySoundAtLocation` (`self.ShootSound`) (`self.K2_GetActorLocation`) (struct) 0.5 1.0 0.0 null null null)
              (if (<= (`self.ShootSoundOffset`) 0.0)
                (`KismetSystemLibrary.Delay` (`KismetMathLibrary.Abs` (`self.ShootSoundOffset`))))
              (`|SpawnActorFromClass` (`self.ProjectileType`) (`KismetMathLibrary.MakeTransform` _returnvalue_location) "AlwaysSpawn" "OverrideRootScale" null null))))))))

(event `self.ReceiveAnyDamage`
  (params (Damage :type "Float (single-precision)") (DamageType :type "DamageType Object Reference") (InstigatedBy :type "Controller Object Reference") (DamageCauser :type "Actor Object Reference"))
  ;[1 1 1] On any damage received
  (bind _enemy_killed (`self.Damage Enemy Fn` Damage))
  (if _enemy_killed
    (`self.Play Animation and Kill Enemy Fn`)))

(event `self.ReceiveHit`
  (params (MyComp :type "PrimitiveComponent Object Reference") (Other :type "Actor Object Reference") (OtherComp :type "PrimitiveComponent Object Reference") (bSelfMoved :type Boolean) (HitLocation :type "Vector Structure") (HitNormal :type "Vector Structure") (NormalImpulse :type "Vector Structure") (Hit :type "HitResult Structure (by ref)"))
  ;[1 1 1] On Hit
  (cast `/Game/Blueprints/Projectiles/BP_ProjectilePlayerBase` Other
    (:`CastFailed`
      (set `self.MoveDirection` (not (`self.MoveDirection`)))
      (bind _asbp_mn2player (cast `/Game/Blueprints/BP_MN2Player` Other))
      (`GameplayStatics.ApplyDamage` _asbp_mn2player (/ (`self.CurrentHealth`) 2.0))
      (`self.Play Animation and Kill Enemy Fn`))))

(fn `Damage Enemy Fn`
  (params (`Damage amount` :type "Float (double-precision)"))
  (returns (`Enemy killed` :type Boolean))
  (set `self.CurrentHealth` (`KismetMathLibrary.FClamp` (- (`self.CurrentHealth`) `Damage amount`) 0.0 (`self.MaxHealth`)))
  (return (<= (`self.CurrentHealth`) 0.0)))

(fn `Play Animation and Kill Enemy Fn`
  (bind _bp_gamemode (`self.BP_GameMode`))
  (`GameplayStatics.SpawnEmitterAtLocation` "/Game/Assets/Particles/P_Pixel_Explosion_Enemy.P_Pixel_Explosion_Enemy" (`self.K2_GetActorLocation`))
  (`/Game/Blueprints/BP_MN2GameMode.Increment Killed Enemies Counter Fn` _bp_gamemode)
  (`/Game/Blueprints/BP_MN2GameMode.UpdateScore` _bp_gamemode (`self.EnemyScoreValue`))
  (`GameplayStatics.PlaySoundAtLocation` "/Game/Assets/SoundFX/explosion.explosion" (`self.K2_GetActorLocation`) (struct) 1.0 1.0 0.0 null null null)
  (`self.K2_DestroyActor`))

(fn `UserConstructionScript`
  (set `self.CurrentHealth` (`self.MaxHealth`)))