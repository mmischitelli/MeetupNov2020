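; BP_EnemyAsteroid is an asteroid enemy that travels straight down the world Z axis once it is activated.
; The PlaySpawnAnimationFn event turns on movement without playing any animation here, and Tick then moves the actor by MoveSpeed scaled by delta time, with sweep enabled.
; The construction script sets the enemy mesh's world scale from a Scale variable.
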(event `self.PlaySpawnAnimationFn`
  (set `self.MoveEnable` true))

(event `self.ReceiveTick`
  (params (DeltaSeconds :type "Float (single-precision)"))
  ;[1 1 1] Movement
  (if (`self.MoveEnable`)
    (`self.K2_SetActorLocation` (+ (`self.K2_GetActorLocation`) (* (`KismetMathLibrary.MakeVector` 0.0 0.0 (* (`self.MoveSpeed`) -1.0)) DeltaSeconds)) true)))

(fn `UserConstructionScript`
  (`parent.UserConstructionScript`)
  (`SceneComponent.SetWorldScale3D` (`self.EnemyMesh`) (`self.Scale`)))