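; BP_HealthBoost is a health pickup actor that acts on BP_MN2Player when something overlaps its Cube component.
; For the player, it passes a value derived from HealthAmount into ApplyDamage, reusing the damage pipeline for the boost, and plays a pickup sound at its location.
; The actor destroys itself after any overlap, including one by a non-player actor.
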(event `self.Cube.OnComponentBeginOverlap`
  (params (OverlappedComponent :type "PrimitiveComponent Object Reference") (OtherActor :type "Actor Object Reference") (OtherComp :type "PrimitiveComponent Object Reference") (OtherBodyIndex :type Integer) (bFromSweep :type Boolean) (SweepResult :type "HitResult Structure (by ref)"))
  (bind _asbp_mn2player (cast `/Game/Blueprints/BP_MN2Player` OtherActor)
    (:`then`
      (bind _result (`/Engine/EditorBlueprintResources/StandardMacros.NegateFloat` (`self.HealthAmount`))
        (:`  `
          (`GameplayStatics.ApplyDamage` _asbp_mn2player _result)
          (`GameplayStatics.PlaySoundAtLocation` "/Game/Assets/SoundFX/health_pickup.health_pickup" (`self.K2_GetActorLocation`) (struct) 1.0 1.0 0.0 null null null))))
    (:`CastFailed`
      _))
  (`self.K2_DestroyActor`))

(fn `UserConstructionScript`
  (`parent.UserConstructionScript`))