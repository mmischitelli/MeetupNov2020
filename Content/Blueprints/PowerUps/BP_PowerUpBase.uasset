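; BP_PowerUpBase is a base power-up actor: a cube mesh moved by a ProjectileMovement component, with variables for color, scale and speed.
; The construction script creates a dynamic material on the cube, applies the mesh scale, and sets both initial and max projectile speed from the movement speed.
; BeginPlay writes the actor color into the material's Color parameter; the file implements no overlap or pickup logic.
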(event `self.ReceiveBeginPlay`
  (`MaterialInstanceDynamic.SetVectorParameterValue` (`self.ActorMaterial`) "Color" (`self.ActorColor`)))

(fn `UserConstructionScript`
  (bind _projectilemovement (`self.ProjectileMovement`))
  (bind _returnvalue (`PrimitiveComponent.CreateDynamicMaterialInstance` (`self.Cube`) 0 null "None"))
  (set `self.ActorMaterial` _returnvalue)
  (`SceneComponent.SetWorldScale3D` (`self.Cube`) (`self.MeshScale`))
  (bind _output_get (set `ProjectileMovementComponent.MaxSpeed` (`self.MovementSpeed`) _projectilemovement))
  (set `ProjectileMovementComponent.InitialSpeed` _output_get _projectilemovement))